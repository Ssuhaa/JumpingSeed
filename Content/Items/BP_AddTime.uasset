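; Time pickup that adds PlusTime to the game mode's Seconds when BP_PlayerCharacter overlaps its sphere.
; Pickup also activates the player's PTurch, adds a WG_GetTime popup to the timer HUD, updates its warning animation and plays a sound.
; It sets the game mode's GetTime flag to request another clock spawn, then destroys itself.
; The cube spins every tick, and the construction script configures InterpToMovement between two relative points using Speed as duration.
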(event `self.ReceiveBeginPlay`)

(event `self.Sphere.OnComponentBeginOverlap`
  (params (OverlappedComponent :type "PrimitiveComponent Object Reference") (OtherActor :type "Actor Object Reference") (OtherComp :type "PrimitiveComponent Object Reference") (OtherBodyIndex :type Integer) (bFromSweep :type Boolean) (SweepResult :type "HitResult Structure (by ref)"))
  (bind _plustime (`self.PlusTime`))
  (bind _asbp_third_person_game_mode (cast `/Game/ThirdPerson/Blueprints/BP_ThirdPersonGameMode` (`GameplayStatics.GetGameMode`) :!pure true))
  (bind _wg_timer (`/Game/ThirdPerson/Blueprints/BP_ThirdPersonGameMode.WG_Timer` (cast `/Game/ThirdPerson/Blueprints/BP_ThirdPersonGameMode` (`GameplayStatics.GetGameMode`) :!pure true)))
  ;[1 1 1] 획득 시 시간 추가
  (bind _asbp_player_character (cast `/Game/ThirdPerson/Characters/BP_PlayerCharacter` OtherActor))
  (`ActorComponent.Activate` (`/Game/ThirdPerson/Characters/BP_PlayerCharacter.P_Turch` _asbp_player_character) true)
  (set `/Game/ThirdPerson/Blueprints/BP_ThirdPersonGameMode.Seconds` (+ (`/Game/ThirdPerson/Blueprints/BP_ThirdPersonGameMode.Seconds` _asbp_third_person_game_mode) _plustime) _asbp_third_person_game_mode)
  ;[1 1 1] 얻은 시간만큼 애니메이션 재생, 획득했을 때 30초 이상이 되면 애니메이션 재생을 멈춤
  (bind _returnvalue (`|CreateWidget` "/Game/Widget/WG_GetTime.WG_GetTime_C"))
  (set `/Game/Widget/WG_GetTime.Seconds` _plustime _returnvalue)
  (`Overlay.AddChildToOverlay` (`/Game/Widget/WG_Timer.GetTime_Overlay` _wg_timer) _returnvalue)
  (`/Game/Widget/WG_Timer.Warning Animation` _wg_timer)
  ;;[1 1 1] 획득 시 다른 곳에 또 다른 시계 추가 스폰
  (set `/Game/ThirdPerson/Blueprints/BP_ThirdPersonGameMode.Get Time?` true (cast `/Game/ThirdPerson/Blueprints/BP_ThirdPersonGameMode` (`GameplayStatics.GetGameMode`) :!pure true))
  (`GameplayStatics.PlaySound2D` "/Game/Sound/SFX/sc_FX_GetTime.sc_FX_GetTime" 1.0 1.0 0.0 null null)
  (`self.K2_DestroyActor`))

(event `self.ReceiveTick`
  (params (DeltaSeconds :type "Float (single-precision)"))
  (`SceneComponent.K2_AddLocalRotation` (`self.Cube`) (struct :`Yaw` 1.0) false false))

(fn `UserConstructionScript`
  (bind _interptomovement (`self.InterpToMovement`))
  (set `InterpToMovementComponent.ControlPoints` (`|MakeArray` (make `InterpControlPoint` (`self.Location_1`)) (make `InterpControlPoint` (`self.Location_2`))) _interptomovement)
  (set `InterpToMovementComponent.Duration` (`self.Speed`) _interptomovement))