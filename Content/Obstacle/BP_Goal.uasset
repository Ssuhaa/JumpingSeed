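; BP_Goal is the finish-line trigger that ends a run successfully when the player character overlaps its Box.
; It shows the WG_GameSuccess widget, flags success on Gameinstance1, passes the game mode's FastSeconds to ResultTime, then opens the Result level after a short delay.
; A second Sequence branch removes the game mode's timer widget without waiting for that delay.
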(event `self.ReceiveBeginPlay`)

(event `self.Box.OnComponentBeginOverlap`
  (params (OverlappedComponent :type "PrimitiveComponent Object Reference") (OtherActor :type "Actor Object Reference") (OtherComp :type "PrimitiveComponent Object Reference") (OtherBodyIndex :type Integer) (bFromSweep :type Boolean) (SweepResult :type "HitResult Structure (by ref)"))
  (bind _asgameinstance_1 (cast `/Game/ThirdPerson/Blueprints/Gameinstance1` (`GameplayStatics.GetGameInstance`) :!pure true))
  ;[1 1 1] 골인 시 성공 위젯 생성, 현재 기록 저장
  (cast `/Game/ThirdPerson/Characters/BP_PlayerCharacter` OtherActor)
  (`|ExecutionSequence`
    (:`then_0`
      (bind _returnvalue (`|CreateWidget` "/Game/Widget/WG_GameSuccess.WG_GameSuccess_C"))
      (`UserWidget.AddToViewport` _returnvalue 0)
      (set `/Game/ThirdPerson/Blueprints/Gameinstance1.Success?` true _asgameinstance_1)
      (`/Game/ThirdPerson/Blueprints/Gameinstance1.result Time` _asgameinstance_1 (`/Game/ThirdPerson/Blueprints/BP_ThirdPersonGameMode.Fast Seconds` (cast `/Game/ThirdPerson/Blueprints/BP_ThirdPersonGameMode` (`GameplayStatics.GetGameMode`) :!pure true)))
      (`KismetSystemLibrary.Delay` 2.0)
      (`GameplayStatics.OpenLevel` "Result"))
    (:`then_1`
      (`Widget.RemoveFromParent` (`/Game/ThirdPerson/Blueprints/BP_ThirdPersonGameMode.WG_Timer` (cast `/Game/ThirdPerson/Blueprints/BP_ThirdPersonGameMode` (`GameplayStatics.GetGameMode`) :!pure true))))))

(fn `UserConstructionScript`)