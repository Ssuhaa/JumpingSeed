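; BP_CushionPad is an obstacle that knocks the player back on contact.
; BeginPlay gives the Cube a random yaw picked from the Rotation array.
; When a BP_PlayerCharacter enters the Box, it starts the DamagedBack montage and immediately launches the character with random X and Y velocities from two arrays and a fixed upward boost.
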(event `self.ReceiveBeginPlay`
  (`SceneComponent.K2_SetRelativeRotation` (`self.Cube`) (`KismetMathLibrary.MakeRotator` 0.0 0.0 (`KismetMathLibrary.Conv_IntToDouble` (`KismetArrayLibrary.Array_Random` (`self.Rotation`)))) false false))

(event `self.Box.OnComponentBeginOverlap`
  (params (OverlappedComponent :type "PrimitiveComponent Object Reference") (OtherActor :type "Actor Object Reference") (OtherComp :type "PrimitiveComponent Object Reference") (OtherBodyIndex :type Integer) (bFromSweep :type Boolean) (SweepResult :type "HitResult Structure (by ref)"))
  (bind _asbp_player_character (cast `/Game/ThirdPerson/Characters/BP_PlayerCharacter` OtherActor))
  (`|PlayMontage` (`Character.Mesh` _asbp_player_character) "/Game/SdMotionPack/Montage/DamagedBack_Montage.DamagedBack_Montage"
    (:`then`
      (`Character.LaunchCharacter` _asbp_player_character (`KismetMathLibrary.MakeVector` (`KismetArrayLibrary.Array_Random` (`self.Launch Velocity X`)) (`KismetArrayLibrary.Array_Random` (`self.Launch Velocity Y`)) 200.0) false false))))

(fn `UserConstructionScript`)