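; BP_PushStick is a moving obstacle that knocks the player character away on contact.
; The construction script builds two relative control points for its InterpToMovement from configurable locations, with Speed as the travel duration, so lower values move faster.
; When the Box overlaps a BP_PlayerCharacter, it plays a slowed damage montage and launches the character with randomly picked X and Y velocities and a fixed upward push.
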(event `self.ReceiveTick`
  (params (DeltaSeconds :type "Float (single-precision)")))

(event `self.Box.OnComponentBeginOverlap`
  (params (OverlappedComponent :type "PrimitiveComponent Object Reference") (OtherActor :type "Actor Object Reference") (OtherComp :type "PrimitiveComponent Object Reference") (OtherBodyIndex :type Integer) (bFromSweep :type Boolean) (SweepResult :type "HitResult Structure (by ref)"))
  ;[1 1 1] Box에 캐릭터 오버랩 시 랜덤한 방향으로 날아감
  (bind _asbp_player_character (cast `/Game/ThirdPerson/Characters/BP_PlayerCharacter` OtherActor))
  (`|PlayMontage` (`Character.Mesh` _asbp_player_character) "/Game/SdMotionPack/Montage/DamagedFront_Montage.DamagedFront_Montage" 0.3
    (:`then`
      (`Character.LaunchCharacter` _asbp_player_character (`KismetMathLibrary.MakeVector` (`KismetArrayLibrary.Array_Random` (`self.Launch Velocity X`)) (`KismetArrayLibrary.Array_Random` (`self.Launch Velocity Y`)) 200.0) true true))))

(fn `UserConstructionScript`
  (bind _interptomovement (`self.InterpToMovement`))
  ;[1 1 1] 설정해놓은 로케이션으로 액터가 계속해서 움직임. Speed가 낮을수록 빠름
  (set `InterpToMovementComponent.ControlPoints` (`|MakeArray` (make `InterpControlPoint` (`self.Location_1`)) (make `InterpControlPoint` (`self.Location_2`))) _interptomovement)
  (set `InterpToMovementComponent.Duration` (`self.Speed`) _interptomovement))