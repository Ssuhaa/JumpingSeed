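; BP_PushBlock is a moving obstacle that hits the player character on contact.
; The construction script gives its InterpToMovement two relative control points, Location1 and Location2, for ping-pong travel, as its comment notes.
; Speed is assigned as the movement Duration, so lower values move the block faster.
; Box overlap with BP_PlayerCharacter plays a hit sound and calls the character's Hit, commented as enabling physics simulation.
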(event `self.ReceiveBeginPlay`)

(event `self.Box.OnComponentBeginOverlap`
  (params (OverlappedComponent :type "PrimitiveComponent Object Reference") (OtherActor :type "Actor Object Reference") (OtherComp :type "PrimitiveComponent Object Reference") (OtherBodyIndex :type Integer) (bFromSweep :type Boolean) (SweepResult :type "HitResult Structure (by ref)"))
  ;[1 1 1] Box에 캐릭터 오버랩 시 캐릭터 Physics Simulate 켜기
  (bind _asbp_player_character (cast `/Game/ThirdPerson/Characters/BP_PlayerCharacter` OtherActor))
  (`GameplayStatics.PlaySoundAtLocation` "/Game/Sound/SFX/sc_FX_Hit.sc_FX_Hit" (`self.K2_GetActorLocation` _asbp_player_character) (struct) 1.0 1.0 0.0 null null null null)
  (`/Game/ThirdPerson/Characters/BP_PlayerCharacter.Hit` _asbp_player_character))

(fn `UserConstructionScript`
  (bind _interptomovement (`self.InterpToMovement`))
  ;[1 1 1] 정해둔 로케이션으로 액터가 PingPong 방식으로 이동. Speed가 낮을수록 빠름.
  (set `InterpToMovementComponent.ControlPoints` (`|MakeArray` (make `InterpControlPoint` (`self.Location_1`)) (make `InterpControlPoint` (`self.Location_2`))) _interptomovement)
  (set `InterpToMovementComponent.Duration` (`self.Speed`) _interptomovement))