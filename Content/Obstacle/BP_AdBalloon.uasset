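; BP_AdBalloon is an advertising balloon obstacle actor that moves up and down.
; Tick accumulates runtime and adds a sine offset, shaped by Speed and Length, to the Balloon component's current relative Z.
; Because the offset accumulates every frame instead of starting from a stored base height, the travel range depends on frame rate.
; The construction script applies the Materials variable to the balloon's first material slot.
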(event `self.ReceiveBeginPlay`)

(event `self.ReceiveTick`
  (params (DeltaSeconds :type "Float (single-precision)"))
  (bind _balloon (`self.Balloon`))
  (bind (_relativelocation_x _relativelocation_y _relativelocation_z) (`KismetMathLibrary.BreakVector` (`SceneComponent.RelativeLocation` _balloon)))
  (bind _output_get (set `self.Runtime` (+ DeltaSeconds (`self.Runtime`))))
  (`SceneComponent.K2_SetRelativeLocation` _balloon (`KismetMathLibrary.MakeVector` _relativelocation_x _relativelocation_y (+ (* (`KismetMathLibrary.Sin` (* _output_get (`self.Speed`))) (`self.length`)) _relativelocation_z)) false false))

(fn `UserConstructionScript`
  (`PrimitiveComponent.SetMaterial` (`self.Balloon`) 0 (`self.Materials`)))