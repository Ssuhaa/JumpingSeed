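; BP_RandomDoor is an obstacle with four doors built from paired cube components, one of which is randomly made passable at start.
; BeginPlay maps each cube to its partner, then picks a random key and enables physics simulation on that cube and its looked-up partner.
; Front and back kill zones destroy overlapping left or right push-box mesh components and play a door explosion sound.
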(event `self.ReceiveBeginPlay`
  (set `self.Cube` (`|MakeMap` (`self.Cube1`) (`self.Cube1_1`) (`self.Cube2`) (`self.Cube2-1`) (`self.Cube3`) (`self.Cube3_1`) (`self.Cube4`) (`self.Cube4_1`)))
  (bind _keys (`BlueprintMapLibrary.Map_Keys` (`self.Cube`)))
  (`PrimitiveComponent.SetSimulatePhysics` (`KismetArrayLibrary.Array_Random` _keys) true)
  (`PrimitiveComponent.SetSimulatePhysics` (`BlueprintMapLibrary.Map_Find` (`self.Cube`) (`KismetArrayLibrary.Array_Random` _keys)) true))

(event `self.BackKillZone.OnComponentBeginOverlap`
  (params (OverlappedComponent :type "PrimitiveComponent Object Reference") (OtherActor :type "Actor Object Reference") (OtherComp :type "PrimitiveComponent Object Reference") (OtherBodyIndex :type Integer) (bFromSweep :type Boolean) (SweepResult :type "HitResult Structure (by ref)"))
  (bind `_as스태틱_메시_컴포넌트` (cast `StaticMeshComponent` OtherComp))
  (bind _staticmesh (`StaticMeshComponent.StaticMesh` `_as스태틱_메시_컴포넌트`))
  (if (or (== _staticmesh "/Game/Geometry/Meshes/SM_PushBox_L.SM_PushBox_L") (== _staticmesh "/Game/Geometry/Meshes/SM_PushBox_R.SM_PushBox_R"))
    (`GameplayStatics.PlaySound2D` "/Game/Sound/SFX/sc_FX_DoorExplosion.sc_FX_DoorExplosion" 1.0 1.0 0.0 null null)
    (`ActorComponent.K2_DestroyComponent` OtherComp)))

(event `self.FrontKillZone.OnComponentBeginOverlap`
  (params (OverlappedComponent :type "PrimitiveComponent Object Reference") (OtherActor :type "Actor Object Reference") (OtherComp :type "PrimitiveComponent Object Reference") (OtherBodyIndex :type Integer) (bFromSweep :type Boolean) (SweepResult :type "HitResult Structure (by ref)"))
  (bind `_as스태틱_메시_컴포넌트` (cast `StaticMeshComponent` OtherComp))
  (bind _staticmesh (`StaticMeshComponent.StaticMesh` `_as스태틱_메시_컴포넌트`))
  (if (or (== _staticmesh "/Game/Geometry/Meshes/SM_PushBox_L.SM_PushBox_L") (== _staticmesh "/Game/Geometry/Meshes/SM_PushBox_R.SM_PushBox_R"))
    (`GameplayStatics.PlaySound2D` "/Game/Sound/SFX/sc_FX_DoorExplosion.sc_FX_DoorExplosion" 1.0 1.0 0.0 null null)
    (`ActorComponent.K2_DestroyComponent` OtherComp)))

(fn `UserConstructionScript`)