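; BP_RollingCircle is an obstacle disc that spins continuously in one of two directions, chosen by the IsRightRotaiton flag.
; BeginPlay gives the Cylinder mesh one of two materials to match the direction.
; Tick adds a fixed positive or negative world rotation each frame without delta-time scaling, so spin speed depends on frame rate.
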(event `self.ReceiveBeginPlay`
  (bind _cylinder (`self.Cylinder`))
  ;[1 1 1] 시작 시 회전하는 방향에 맞는 머터리얼 적용
  (if (`self.is Right Rotaiton?`)
    (`PrimitiveComponent.SetMaterial` _cylinder 0 "/Game/Geometry/Materials/MI_RollingCycle.MI_RollingCycle")
    (else
      (`PrimitiveComponent.SetMaterial` _cylinder 0 "/Game/Geometry/Materials/MI_RollingCycle_2.MI_RollingCycle_2"))))

(event `self.ReceiveTick`
  (params (DeltaSeconds :type "Float (single-precision)"))
  (bind _cylinder (`self.Cylinder`))
  ;[1 1 1] 원판 회전, Bool 체크를 통해 방향을 바꿀 수 있음
  (if (`self.is Right Rotaiton?`)
    (`SceneComponent.K2_AddWorldRotation` _cylinder (struct :`Yaw` 1.0) false false)
    (else
      (`SceneComponent.K2_AddWorldRotation` _cylinder (struct :`Yaw` -1.0) false false))))

(fn `UserConstructionScript`)