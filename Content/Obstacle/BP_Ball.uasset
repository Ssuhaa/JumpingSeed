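; BP_Ball is a physics ball obstacle that knocks the player character back on contact.
; On BeginPlay it shoots itself along negative X with an upward velocity impulse and takes a random material from an array.
; When the ball hits BP_PlayerCharacter, it starts a slowed damage montage and immediately launches the character backward along world X and upward, with a random sideways velocity.
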(event `self.ReceiveBeginPlay`
  (`|ExecutionSequence`
    (:`then_0`
      (`PrimitiveComponent.AddImpulse` (`self.Ball`) (-1000.0 0.0 300.0) "None" true))
    (:`then_1`
      (`PrimitiveComponent.SetMaterial` (`self.Ball`) 0 (`KismetArrayLibrary.Array_Random` (`self.Material`))))))

(event `self.Ball.OnComponentHit`
  (params (HitComponent :type "PrimitiveComponent Object Reference") (OtherActor :type "Actor Object Reference") (OtherComp :type "PrimitiveComponent Object Reference") (NormalImpulse :type "Vector Structure") (Hit :type "HitResult Structure (by ref)"))
  (bind _asbp_player_character (cast `/Game/ThirdPerson/Characters/BP_PlayerCharacter` OtherActor))
  (`|PlayMontage` (`Character.Mesh` _asbp_player_character) "/Game/SdMotionPack/Montage/DamagedFront_Montage.DamagedFront_Montage" 0.3
    (:`then`
      (`Character.LaunchCharacter` _asbp_player_character (`KismetMathLibrary.MakeVector` -300.0 (`KismetArrayLibrary.Array_Random` (`self.Launch Velocity Y`)) 200.0) true true))))

(fn `UserConstructionScript`)