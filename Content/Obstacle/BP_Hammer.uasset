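; BP_Hammer is a rotating hammer obstacle that hits the player character on contact.
; Each Tick it yaws its Scene component by the plus or minus speed chosen by IsPlusRotate, without delta-time scaling.
; When BP_PlayerCharacter overlaps the Box, it plays a hit sound at the hammer's location and calls the character's Hit function, commented as enabling physics simulation.
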(event `self.ReceiveTick`
  (params (DeltaSeconds :type "Float (single-precision)"))
  (bind _scene (`self.Scene`))
  ;[1 1 1] 액터 회전 노드. Bool 체크를 통해 방향을 바꿀 수 있음.
  (if (`self.Is Plus Rotate?`)
    (`SceneComponent.K2_AddLocalRotation` _scene (`KismetMathLibrary.MakeRotator` 0.0 0.0 (`self.Plus Rotate Speed`)) false false)
    (else
      (`SceneComponent.K2_AddLocalRotation` _scene (`KismetMathLibrary.MakeRotator` 0.0 0.0 (`self.Minus Rotate Speed`)) false false))))

(event `self.Box.OnComponentBeginOverlap`
  (params (OverlappedComponent :type "PrimitiveComponent Object Reference") (OtherActor :type "Actor Object Reference") (OtherComp :type "PrimitiveComponent Object Reference") (OtherBodyIndex :type Integer) (bFromSweep :type Boolean) (SweepResult :type "HitResult Structure (by ref)"))
  ;[1 1 1] Box에 오버랩 시 캐릭터 Physics Simulate 켜기
  (bind _asbp_player_character (cast `/Game/ThirdPerson/Characters/BP_PlayerCharacter` OtherActor))
  (`GameplayStatics.PlaySoundAtLocation` "/Game/Sound/SFX/sc_FX_Hit.sc_FX_Hit" (`self.K2_GetActorLocation`) (struct) 1.0 1.0 0.0 null null null null)
  (`/Game/ThirdPerson/Characters/BP_PlayerCharacter.Hit` _asbp_player_character))

(fn `UserConstructionScript`)