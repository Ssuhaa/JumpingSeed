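; BP_SlipperyGround is an obstacle area that makes player characters slide and pushes them in one direction.
; Box overlap begin and end events switch the character's ground friction and jump velocity between slip and normal values held in variables.
; Every Tick, overlapping player characters are moved along the Arrow component's forward vector by Speed times delta time, using an unswept world offset.
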(event `self.Box.OnComponentBeginOverlap`
  (params (OverlappedComponent :type "PrimitiveComponent Object Reference") (OtherActor :type "Actor Object Reference") (OtherComp :type "PrimitiveComponent Object Reference") (OtherBodyIndex :type Integer) (bFromSweep :type Boolean) (SweepResult :type "HitResult Structure (by ref)"))
  ;[1 1 1] Box에 캐릭터 오버랩 시 점프, 마찰력 값 조정
  (bind _asbp_player_character (cast `/Game/ThirdPerson/Characters/BP_PlayerCharacter` OtherActor))
  (bind _charactermovement (`Character.CharacterMovement` _asbp_player_character))
  (set `CharacterMovementComponent.GroundFriction` (`self.Slip Ground Friction`) _charactermovement)
  (set `CharacterMovementComponent.JumpZVelocity` (`self.Slip Jump Z Velocity`) _charactermovement))

(event `self.Box.OnComponentEndOverlap`
  (params (OverlappedComponent :type "PrimitiveComponent Object Reference") (OtherActor :type "Actor Object Reference") (OtherComp :type "PrimitiveComponent Object Reference") (OtherBodyIndex :type Integer))
  ;[1 1 1] Box에 캐릭터 오버랩이 끝나면 점프, 마찰 원래 값으로 초기화
  (bind _asbp_player_character (cast `/Game/ThirdPerson/Characters/BP_PlayerCharacter` OtherActor))
  (bind _charactermovement (`Character.CharacterMovement` _asbp_player_character))
  (set `CharacterMovementComponent.GroundFriction` (`self.NonSlip Ground Friction`) _charactermovement)
  (set `CharacterMovementComponent.JumpZVelocity` (`self.NonSlip Jump Z Velocity`) _charactermovement))

(event `self.ReceiveTick`
  (params (DeltaSeconds :type "Float (single-precision)"))
  ;[1 1 1] 콜리전에 캐릭터 오버랩 시 Arrow 방향으로 밀어냄
  (for _array_element (`PrimitiveComponent.GetOverlappingActors` (`self.Box`) "/Game/ThirdPerson/Characters/BP_PlayerCharacter.BP_PlayerCharacter_C")
    (`self.K2_AddActorWorldOffset` _array_element (* (* DeltaSeconds (`self.Speed`)) (`KismetMathLibrary.GetForwardVector` (`SceneComponent.K2_GetComponentRotation` (`self.Arrow`)))) false false)))

(fn `UserConstructionScript`)