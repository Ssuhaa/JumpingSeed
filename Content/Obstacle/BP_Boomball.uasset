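; BP_Boomball is a cannon obstacle that repeatedly fires BP_Ball actors.
; On BeginPlay it starts a looping timer with an interval picked at random from the Time array (noted as 2–3 seconds), so each instance keeps that interval.
; Each tick of the timer plays a cannon sound, spawns a ball at the Scene component's transform and emits a scaled particle effect there.
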(event `self.ReceiveBeginPlay`
  ;[1 1 1] 2~3초 간격으로 공 발사
  (`KismetSystemLibrary.K2_SetTimerDelegate` (delegate `BallSpwan`) (`KismetArrayLibrary.Array_Random` (`self.Time`)) true))

(event `BallSpwan`
  (bind _scene (`self.Scene`))
  ;[1 1 1] 2~3초 간격으로 공 발사
  (`GameplayStatics.PlaySoundAtLocation` "/Game/Sound/SFX/sc_FX_Cannon.sc_FX_Cannon" (`self.K2_GetActorLocation`) (struct) 1.0 1.0 0.0 null null null null)
  (`|SpawnActorFromClass` "/Game/Obstacle/BP_Ball.BP_Ball_C" (`SceneComponent.K2_GetComponentToWorld` _scene) "Undefined" "OverrideRootScale" null null)
  (`GameplayStatics.SpawnEmitterAtLocation` "/Engine/Tutorial/SubEditors/TutorialAssets/TutorialParticleSystem.TutorialParticleSystem" (`SceneComponent.K2_GetComponentLocation` _scene) (struct :`Pitch` -90.0) (1.5 1.5 1.5)))

(fn `UserConstructionScript`)